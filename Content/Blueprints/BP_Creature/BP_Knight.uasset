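; BP_Knight is a creature Blueprint for an input-controlled Knight that can attack and run.
; On BeginPlay it loads the "Knight" creature data table row into Data before calling parent BeginPlay, which only runs if the row is found.
; It then snaps itself to tile (1,1) of the level's BP_Tilemap if that tile is valid.
; Attack input calls BeginAttack, and holding Run raises the walk speed until released.
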(event EventBeginPlay
  (bind _returnvalue (Utilities|GetDataTableRow "/Game/Blueprints/Data/CreatureDataTable.CreatureDataTable" "Knight")
    (:then
      (Variables|Default|SetData _returnvalue)
      (|CallParentFunction)
      (bind _returnvalue_2 (Actor|GetActorOfClass "/Game/Blueprints/BP_Tilemap.BP_Tilemap_C"))
      (if (.bValid (Default|GetTilePos _returnvalue_2 1 1))
        (Transformation|SetActorLocation (.Location (Default|GetTilePos _returnvalue_2 1 1)) false false)))))

(event EventTick
  (params (DeltaSeconds :type Float%20%28single-precision%29))
  (|CallParentFunction DeltaSeconds))

(event Input|ActionEvents|InputActionAttack
  (params (Key :type Key%20Structure :default "None"))
  (:Pressed
    (CallFunction|BeginAttack)))

(event Input|ActionEvents|InputActionRun
  (params (Key :type Key%20Structure :default "None"))
  (:Pressed
    (Variables|/Script/Engine.CharacterMovementComponent|SetMaxWalkSpeed (Variables|Character|GetCharacterMovement) 1.5e+03))
  (:Released
    (Variables|/Script/Engine.CharacterMovementComponent|SetMaxWalkSpeed (Variables|Character|GetCharacterMovement) 6e+02)))

(fn ConstructionScript)