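; BP_Tilemap is a tilemap actor that serves as a walkability grid for tile-based movement.
; On BeginPlay it sizes a boolean grid from its tilemap and flags cells holding a layer 1 tile as blocked, assuming a hardcoded width of 10.
; CanGo reports whether an in-range cell is free.
; GetTilePos converts grid coordinates to world locations on the XZ plane, with both using GridPosToIndex for bounds checks.
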(event EventBeginPlay
  (bind _rendercomponent (Variables|Default|GetRenderComponent))
  (bind _tilemap (Variables|/Script/Paper2D.PaperTileMapComponent|GetTileMap _rendercomponent))
  (Utilities|FlowControl|Sequence
    (:then_0
      (Utilities|Array|Resize (Variables|Default|GetMapGrid) (* (Variables|/Script/Paper2D.PaperTileMap|GetMapWidth _tilemap) (Variables|/Script/Paper2D.PaperTileMap|GetMapHeight _tilemap)))
      (Variables|Default|SetMapWidth (Variables|/Script/Paper2D.PaperTileMap|GetMapWidth _tilemap))
      (Variables|Default|SetMapHeight (Variables|/Script/Paper2D.PaperTileMap|GetMapHeight _tilemap)))
    (:then_1
      (for (_ _array_index) (Variables|Default|GetMapGrid)
        (Utilities|IsValid (.tileset (Class|PaperTileMapComponent|GetTile (Variables|Default|GetRenderComponent) (Math|Integer|%(Integer) _array_index 10) (/ _array_index 10) 1))
          (:Is%20Valid
            (Utilities|Array|SetArrayElem (Variables|Default|GetMapGrid) _array_index true)))))))

(fn ConstructionScript)

(fn CanGo
  (params (GridX :type Integer) (GridY :type Integer))
  (bind (_bvalid _index) (CallFunction|GridPostoIndex GridX GridY))
  (if _bvalid
    (return (not (Utilities|Array|Get(acopy) (Variables|Default|GetMapGrid) _index)))
    (else
      (return false))))

(fn GridPostoIndex
  (params (GridX :type Integer) (GridY :type Integer))
  (return (and (Math|Integer|InRange(Integer) GridX 0 (Variables|Default|GetMapWidth) true false) (Math|Integer|InRange(Integer) GridY 0 (Variables|Default|GetMapHeight) true false)) (+ (* GridY (Variables|Default|GetMapWidth)) GridX)))

(fn GetTilePos
  (params (GridX :type Integer) (GridY :type Integer))
  (bind _bvalid (CallFunction|GridPostoIndex GridX GridY))
  (return _bvalid (+ (Transformation|GetActorLocation) (Math|Vector|MakeVector (* 5 (* GridX (Variables|Default|GetMapSizeX))) 0.0 (* -5 (* GridY (Variables|Default|GetMapSizeY)))))))