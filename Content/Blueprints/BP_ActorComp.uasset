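; Actor component that keeps spawning skeleton creatures on its owning BP_Tilemap.
; On BeginPlay it caches the owner as the tilemap and starts a self-rescheduling spawn loop, doing nothing if the cast fails.
; Below the creature cap, it increments the count, waits a short random delay, then asks the tilemap to spawn a BP_Skeleton.
; At the cap it polls on a fixed delay; this graph never decrements the count.
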(event Custom|TickRandomSpawn
  (if (< (Variables|Default|GetCreatureCount) (Variables|Default|GetMaxCreatureCount))
    (Math|Integer|IncrementInt (Variables|Default|GetCreatureCount)
      (:%20%20
        (Utilities|FlowControl|Delay (Math|Random|RandomFloatinRange 0.0 5.0))
        (Default|SpawnCreature (Variables|Default|GetTileMap) "/Game/Blueprints/BP_Creature/BP_Skeleton.BP_Skeleton_C")
        (CallFunction|TickRandomSpawn)))
    (else
      (Utilities|FlowControl|Delay 1.0)
      (CallFunction|TickRandomSpawn))))

(event EventBeginPlay
  (bind _asbp_tilemap (Utilities|Casting|CastToBP_Tilemap (Components|GetOwner)))
  (Variables|Default|SetTileMap _asbp_tilemap)
  (CallFunction|TickRandomSpawn))